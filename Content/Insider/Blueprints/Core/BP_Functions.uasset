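; Blueprint function library of shared helpers for player state, UI and mesh setup.
; GetPlayer finds the core player actor among the pawn's child actors, feeding helpers that toggle input, set movement and control types, and update inventory items' interactivity and prompts.
; Other helpers show a single replaceable notice, open the interaction widget as an inventory, convert seconds into timeline play rates, and apply data-driven meshes with optional dynamic materials.
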(fn `GetPlayer`
  (returns (`As Core Engine` :type "Object Object Reference"))
  (bind _filteredarray (`KismetArrayLibrary.FilterArray` (`Actor.GetAllChildActors` (`GameplayStatics.GetPlayerPawn` null) true)))
  (bind _asbp_core_engine (cast `` (`|GetArrayItem` _filteredarray))
    (:`then`
      (return _asbp_core_engine))
    (:`CastFailed`
      (`KismetSystemLibrary.PrintString` null "Attach CoreEngine To Player's Camera"))))

(fn `Notice`
  (params (FrontMessage :type Text) (BoldMessage :type Text) (Message :type Text))
  (bind _foundwidgets (`WidgetBlueprintLibrary.GetAllWidgetsOfClass` null "/Game/Insider/Blueprints/UI/Notice/WBP_Notice.WBP_Notice_C" false))
  (`Widget.RemoveFromParent` _foundwidgets)
  (bind _returnvalue (`|CreateWidget` "/Game/Insider/Blueprints/UI/Notice/WBP_Notice.WBP_Notice_C" null FrontMessage BoldMessage Message))
  (`UserWidget.AddToViewport` _returnvalue 1))

(fn `OpenInventory`
  (bind _returnvalue (`|CreateWidget` "/Game/Insider/Blueprints/UI/Interaction/WBP_Interaction.WBP_Interaction_C"))
  (set `/Game/Insider/Blueprints/UI/Interaction/WBP_Interaction.Inspection` false _returnvalue)
  (`UserWidget.AddToViewport` _returnvalue 0))

(fn `PlayerControl`
  (params (`Movement Type` :type "/Game/Insider/Blueprints/Core/Enums/Enum_MovementType Enum" :default "NewEnumerator0") (`Control Type` :type "/Game/Insider/Blueprints/Events/Enums/Enum_GE_ControlType Enum" :default "NewEnumerator1"))
  (`self.PlayerInput` true `Movement Type`)
  (bind _as_core_engine (`self.GetPlayer` null))
  (set `/Game/Insider/Blueprints/Core/BP_Functions.CurrentControlType` `Control Type` _as_core_engine))

(fn `PlayerInput`
  (params (Enabled :type Boolean) (`Movement (if enabled)` :type "/Game/Insider/Blueprints/Core/Enums/Enum_MovementType Enum" :default "NewEnumerator0"))
  (bind _returnvalue (`GameplayStatics.GetPlayerPawn` null))
  (bind _returnvalue_2 (`GameplayStatics.GetPlayerController` null))
  (bind _as_core_engine (`self.GetPlayer` null))
  (if Enabled
    (`Actor.EnableInput` _returnvalue _returnvalue_2)
    (`Actor.EnableInput` _as_core_engine _returnvalue_2)
    (switch `/Game/Insider/Blueprints/Core/Enums/Enum_MovementType` `Movement (if enabled)`
      (:`NewEnumerator0`
        (set `/Game/Insider/Blueprints/Core/BP_Functions.Running` false _as_core_engine)
        (set `/Game/Insider/Blueprints/Core/BP_Functions.Crouching` false _as_core_engine)
        (set `/Game/Insider/Blueprints/Core/BP_Functions.Walking` true _as_core_engine)
        (set `/Game/Insider/Blueprints/Core/BP_Functions.CurrentMovementType` "NewEnumerator0" _as_core_engine))
      (:`NewEnumerator1`
        (set `/Game/Insider/Blueprints/Core/BP_Functions.Running` false _as_core_engine)
        (set `/Game/Insider/Blueprints/Core/BP_Functions.Crouching` true _as_core_engine)
        (set `/Game/Insider/Blueprints/Core/BP_Functions.Walking` false _as_core_engine)
        (set `/Game/Insider/Blueprints/Core/BP_Functions.CurrentMovementType` "NewEnumerator1" _as_core_engine))
      (:`NewEnumerator2`
        (set `/Game/Insider/Blueprints/Core/BP_Functions.Running` true _as_core_engine)
        (set `/Game/Insider/Blueprints/Core/BP_Functions.Crouching` false _as_core_engine)
        (set `/Game/Insider/Blueprints/Core/BP_Functions.Walking` false _as_core_engine)
        (set `/Game/Insider/Blueprints/Core/BP_Functions.CurrentMovementType` "NewEnumerator2" _as_core_engine)))
    (`self.CalculateSpeed` _as_core_engine)
    (else
      (`Actor.DisableInput` _returnvalue _returnvalue_2)
      (`Actor.DisableInput` _as_core_engine _returnvalue_2)
      (set `/Game/Insider/Blueprints/Core/BP_Functions.Running` false _as_core_engine)
      (set `/Game/Insider/Blueprints/Core/BP_Functions.Crouching` false _as_core_engine)
      (set `/Game/Insider/Blueprints/Core/BP_Functions.Walking` false _as_core_engine))))

(fn `PlayRate`
  (params (Timeline :type "TimelineComponent Object Reference") (Sec :type "Float (double-precision)"))
  (`/Engine/EditorBlueprintResources/StandardMacros.IsValid` Timeline
    (:`Is Valid`
      (`TimelineComponent.SetPlayRate` Timeline (/ 1.0 (select `bool` (<= Sec 0.0) :`false` Sec :`true` 0.001))))))

(fn `SetFilteredItems`
  (params (FilterClass :type "Actor Class Reference") (Interactable :type Boolean) (ChangeInteractionText :type Boolean) (`New Interaction Text` :type Text))
  (bind _as_core_engine (`self.GetPlayer` null))
  (bind _filteredarray (`KismetArrayLibrary.FilterArray` (`/Game/Insider/Blueprints/Core/BP_Functions.PlayerInventory` _as_core_engine) FilterClass))
  (for _array_element _filteredarray
    (bind _asbp_inspectable (cast `` _array_element))
    (set `/Game/Insider/Blueprints/Core/BP_Functions.Interactable` Interactable _asbp_inspectable)
    (bind (_interactionbutton_buttontext _interactionbutton_buttonimage) (break `/Game/Insider/Blueprints/Core/Structs/Struct_ButtonSettings` (`/Game/Insider/Blueprints/Core/BP_Functions.InteractionButton` _asbp_inspectable)))
    (set `/Game/Insider/Blueprints/Core/BP_Functions.InteractionButton` (make `/Game/Insider/Blueprints/Core/Structs/Struct_ButtonSettings` (select `bool` ChangeInteractionText :`false` _interactionbutton_buttontext :`true` `New Interaction Text`) _interactionbutton_buttonimage) _asbp_inspectable)))

(fn `SetMesh`
  (params (StaticMeshComponent :type "StaticMeshComponent Object Reference") (`Mesh Settings` :type "/Game/Insider/Blueprints/UsableAssets/Structs/Struct_SetMesh Structure"))
  (bind (_mesh _materialsettings) (break `/Game/Insider/Blueprints/UsableAssets/Structs/Struct_SetMesh` `Mesh Settings`))
  (`/Engine/EditorBlueprintResources/StandardMacros.IsValid` _mesh
    (:`Is Valid`
      (`StaticMeshComponent.SetStaticMesh` StaticMeshComponent _mesh)
      (if (`KismetArrayLibrary.Array_IsValidIndex` _materialsettings)
        (for _array_element _materialsettings
          (bind (_setmaterial _elemetnid _material _dynamicmaterial _dynamictexture _dynamiccolor _dynamicemissive) (break `/Game/Insider/Blueprints/UsableAssets/Structs/Struct_MaterialSettings` _array_element))
          (if _setmaterial
            (if _dynamicmaterial
              (bind _returnvalue (`PrimitiveComponent.CreateDynamicMaterialInstance` StaticMeshComponent _elemetnid _material "None"))
              (bind (_settexture _parametername _value) (break `/Game/Insider/Blueprints/UsableAssets/Structs/Struct_MS_Texture` _dynamictexture))
              (if _settexture
                (`MaterialInstanceDynamic.SetTextureParameterValue` _returnvalue _parametername _value))
              (bind (_setcolor _parametername_2 _value_2) (break `/Game/Insider/Blueprints/UsableAssets/Structs/Struct_MS_Color` _dynamiccolor))
              (if _setcolor
                (`MaterialInstanceDynamic.SetVectorParameterValue` _returnvalue _parametername_2 _value_2))
              (bind (_setemissive _parametername_3 _value_3) (break `/Game/Insider/Blueprints/UsableAssets/Structs/Struct_MS_Emissive` _dynamicemissive))
              (if _setemissive
                (`MaterialInstanceDynamic.SetScalarParameterValue` _returnvalue _parametername_3 _value_3))
              (else
                (`PrimitiveComponent.SetMaterial` StaticMeshComponent _elemetnid _material)))
            (else
              (break))))))))