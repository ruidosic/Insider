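; Player character that turns input into look, movement, jumping, flashlight and use actions, delegating state and interactions to a Core object from GetPlayer.
; Core's control type selects axis-driven movement (Full Control) or automatic forward movement on Tick (Turn with Look Control), both triggering footstep headshake.
; After teleporting through a tilted portal, a timeline lerps actor and control rotation upright toward the target portal's horizontal forward.
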(event `self.ReceiveBeginPlay`
  (`parent.ReceiveBeginPlay`)
  (bind _as_core_engine (`/Game/Insider/Blueprints/Core/BP_Functions.GetPlayer`))
  (set `self.Core` _as_core_engine))

(event `InputAxis|LookUp`
  (params (AxisValue :type "Float (single-precision)"))
  (`self.AddControllerPitchInput` AxisValue))

(event `InputAxis|Turn`
  (params (AxisValue :type "Float (single-precision)"))
  (`self.AddControllerYawInput` AxisValue))

(event `InputAxis|LookUpRate`
  (params (AxisValue :type "Float (single-precision)"))
  (`self.AddControllerPitchInput` (* AxisValue (`GameplayStatics.GetWorldDeltaSeconds`) (`/Game/Insider/Blueprints/Core/BP_CoreEngine.BaseLookUpRate` (`self.Core`)))))

(event `InputAxis|TurnRate`
  (params (AxisValue :type "Float (single-precision)"))
  (`self.AddControllerYawInput` (* AxisValue (`GameplayStatics.GetWorldDeltaSeconds`) (`/Game/Insider/Blueprints/Core/BP_CoreEngine.BaseTurnRate` (`self.Core`)))))

(event `InputAxis|MoveForward`
  (params (AxisValue :type "Float (single-precision)"))
  (bind _core (`self.Core`))
  (if (or (`/Game/Insider/Blueprints/Core/BP_CoreEngine.Crouching` _core) (`/Game/Insider/Blueprints/Core/BP_CoreEngine.Walking` _core) (`/Game/Insider/Blueprints/Core/BP_CoreEngine.Running` _core))
    (switch `/Game/Insider/Blueprints/Events/Enums/Enum_GE_ControlType` (`/Game/Insider/Blueprints/Core/BP_CoreEngine.CurrentControlType` _core)
      (:`NewEnumerator2`
        (`self.AddMovementInput` (`KismetMathLibrary.GetForwardVector` (`KismetMathLibrary.MakeRotator` 0.0 0.0 (.yaw (`self.GetControlRotation`)))) AxisValue)
        (`/Game/Insider/Blueprints/Core/BP_CoreEngine.Footstep/Headshake` (`self.Core`) "NewEnumerator0" :!label _label)))))

(event `InputAxis|MoveRight`
  (params (AxisValue :type "Float (single-precision)"))
  (bind _core (`self.Core`))
  (if (`NavMovementComponent.IsFlying` (`self.CharacterMovement`))
    _
    (elif (or (`/Game/Insider/Blueprints/Core/BP_CoreEngine.Crouching` _core) (`/Game/Insider/Blueprints/Core/BP_CoreEngine.Running` _core) (`/Game/Insider/Blueprints/Core/BP_CoreEngine.Walking` _core))
      (switch `/Game/Insider/Blueprints/Events/Enums/Enum_GE_ControlType` (`/Game/Insider/Blueprints/Core/BP_CoreEngine.CurrentControlType` _core)
        (:`NewEnumerator2`
          (`self.AddMovementInput` (`KismetMathLibrary.GetRightVector` (`KismetMathLibrary.MakeRotator` 0.0 0.0 (.yaw (`self.GetControlRotation`)))) AxisValue)
          (goto _label))))))

(event `InputAction|Use`
  (params (Key :type "Key Structure"))
  (:`Pressed`
    (`/Game/Insider/Blueprints/Core/BP_CoreEngine.UseHitActor` (`self.Core`))))

(event `Key|Two`
  (params (Key :type "Key Structure"))
  (:`Pressed`
    (`/Game/Insider/Blueprints/Core/BP_CoreEngine.EquipFlashlight` (`self.Core`) false)))

(event `InputAction|Alternative`
  (params (Key :type "Key Structure"))
  (:`Pressed`
    (`/Game/Insider/Blueprints/Core/BP_CoreEngine.AlternativeUseHitActor` (`self.Core`))))

(event `InputAction|Jump`
  (params (Key :type "Key Structure"))
  (:`Pressed`
    (`self.Jump` :!label _label_2)
    (`/Game/Insider/Blueprints/Core/BP_CoreEngine.StartFallingTimer` (`self.Core`))))

(event `self.OnLanded`
  (params (Hit :type "HitResult Structure (by ref)"))
  (`/Game/Insider/Blueprints/Core/BP_CoreEngine.Footstep/Headshake` (`self.Core`) "NewEnumerator1"))

(event `ChangeRotationAnim`
  (params (Rotation :type "Rotator Structure"))
  (bind _returnvalue (`GameplayStatics.GetPlayerController` 0))
  (bind (_direction _animation) (`Timeline|Timeline_1` :!via `PlayFromStart`)
    (:`Update`
      (`self.K2_SetActorRotation` (`KismetMathLibrary.RLerp` (`self.K2_GetActorRotation`) Rotation _animation true) true)
      (`Controller.SetControlRotation` _returnvalue (`KismetMathLibrary.RLerp` (`Controller.GetControlRotation` _returnvalue) Rotation _animation true)))))

(event `CharacterMovementInterface.JumpEvent`
  (params (JumpZ :type "Float (single-precision)"))
  (set `CharacterMovementComponent.JumpZVelocity` JumpZ (`self.CharacterMovement`))
  (goto _label_2))

(event `CharacterMovementInterface.RotationAfterTeleport`
  (params (CurrentPortal :type "Actor Object Reference") (TargetPortal :type "Actor Object Reference"))
  (if (or (not (== (`self.GetActorUpVector` CurrentPortal) (0.0 0.0 1.0))) (not (== (`self.GetActorUpVector` TargetPortal) (0.0 0.0 1.0))))
    (`self.ChangeRotationAnim` (`KismetMathLibrary.MakeRotFromX` (`KismetMathLibrary.MakeVector` (.x (`self.GetActorForwardVector` TargetPortal)) (.y (`self.GetActorForwardVector` TargetPortal)))))))

(event `self.ReceiveTick`
  (params (DeltaSeconds :type "Float (single-precision)"))
  (bind _core (`self.Core`))
  (`parent.ReceiveTick` DeltaSeconds)
  (if (or (`/Game/Insider/Blueprints/Core/BP_CoreEngine.Crouching` _core) (`/Game/Insider/Blueprints/Core/BP_CoreEngine.Walking` _core) (`/Game/Insider/Blueprints/Core/BP_CoreEngine.Running` _core))
    (switch `/Game/Insider/Blueprints/Events/Enums/Enum_GE_ControlType` (`/Game/Insider/Blueprints/Core/BP_CoreEngine.CurrentControlType` (`self.Core`))
      (:`NewEnumerator1`
        (`self.AddMovementInput` (`self.GetActorForwardVector`))
        (`/Game/Insider/Blueprints/Core/BP_CoreEngine.Footstep/Headshake` (`self.Core`) "NewEnumerator0")))))

(fn `UserConstructionScript`
  (`parent.UserConstructionScript`))