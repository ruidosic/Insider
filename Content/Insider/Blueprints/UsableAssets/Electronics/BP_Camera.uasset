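; BP_Camera is a usable security camera that can be switched on or off and reports player detection to an optional control panel.
; A ping-pong timeline sweeps the pivot with randomized speed and pauses between turns.
; A scene capture feeds a render target created at BeginPlay.
; Switching updates mesh, rotation, capture and child BP_Detection sensing; switching and detection also trigger game event checks.
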(event `self.ReceiveBeginPlay`
  ;[1 1 1] Begin Play
  (`self.CreateRenderTarget`))

(event `PlayerDetected`
  ;[1 1 1] Player Detected
  (`self.GameEventCheck` "NewEnumerator32")
  (if (`KismetSystemLibrary.IsValid` (`self.ConrolPanel`))
    (`/Game/Insider/Blueprints/UsableAssets/Electronics/BP_KeyboardControl.PlayerDetected` (`self.ConrolPanel`))))

(event `CameraRotation`
  ;[1 1 1] Camera Rotation
  (if (`self.RotateAnimation`)
    (if (`self.On / Off`)
      (`/Game/Insider/Blueprints/Core/BP_Functions.PlayRate` (`self.CameraRotationTimeline`) (`KismetMathLibrary.RandomFloatInRange` (`self.RotationSpeedMin (Sec)`) (`self.RotationSpeedMax (Sec)`)))
      (if (`self.ReverseRotation`)
        (bind (_direction _animation) (`Timeline|CameraRotationTimeline` :!label _label)
          (:`Update`
            (`SceneComponent.K2_SetRelativeRotation` (`self.CameraPivot`) (`KismetMathLibrary.RLerp` (`self.StartRotation`) (`self.EndRotation`) _animation) false false))
          (:`Finished`
            (if (`self.ReverseRotation`)
              (set `self.ReverseRotation` false)
              (else
                (set `self.ReverseRotation` true)))
            (`KismetSystemLibrary.Delay` (`KismetMathLibrary.RandomFloatInRange` (`self.RotationDelayMin (Sec)`) (`self.RotationDelayMax (Sec)`)))
            (`self.CameraRotation`)))
        (else
          (goto _label :!via `Reverse`)))
      (else
        (goto _label :!via `Stop`)))))

(event `RandomSwitch`
  ;[1 1 1] Camera Rotation
  (if (`self.ReverseRotation`)
    (set `self.ReverseRotation` false)
    (else
      (set `self.ReverseRotation` true)))
  (`self.CameraRotation`))

(event `self.Open/On`
  (params (GameEvent :type Boolean))
  ;[1 1 1] On / Off Events
  (set `self.On / Off` true)
  (`/Game/Insider/Blueprints/Core/BP_Functions.SetMesh` (`self.Camera`) (select `bool` (`self.On / Off`) :`false` (`self.SecurityCamOff`) :`true` (`self.SecurityCamOn`)) :!label _label_2)
  (`self.CameraRotation`)
  (`PawnSensingComponent.SetSensingUpdatesEnabled` (`/Game/Insider/Blueprints/Core/BP_Detection.Detection` (`self.DetectionRef`)) (and (`self.On / Off`) (`self.DetectPlayer`)))
  (set `SceneCaptureComponent.bCaptureEveryFrame` (`self.On / Off`) (`self.CameraCapture`))
  (`self.GameEventCheck` (select `bool` (`self.On / Off`) :`false` "NewEnumerator1" :`true` "NewEnumerator2" :!type "/Game/Insider/Blueprints/Events/Enums/Enum_GameEventCheck Enum")))

(event `self.Close/Off`
  (params (GameEvent :type Boolean))
  ;[1 1 1] On / Off Events
  (set `self.On / Off` false)
  (goto _label_2))

(event `self.Use`
  (params (GameEvent :type Boolean))
  ;[1 1 1] Interaction (Use Event)
  (if (`self.On / Off`)
    (`self.Close/Off` false)
    (else
      (`self.Open/On` false))))

(fn `CreateRenderTarget`
  (bind _returnvalue (`KismetRenderingLibrary.CreateRenderTarget2D` 256 256 "RTF_RGBA8"))
  (bind _output_get (set `SceneCaptureComponent2D.TextureTarget` _returnvalue (`self.CameraCapture`)))
  (set `self.RenderTarget` _output_get)
  (set `SceneCaptureComponent2D.FOVAngle` (`self.SecurityCamFOV`) (`self.CameraCapture`))
  (`/Game/Insider/Blueprints/Core/BP_Functions.SetMesh` (`self.Camera`) (select `bool` (`self.On / Off`) :`false` (`self.SecurityCamOff`) :`true` (`self.SecurityCamOn`)))
  (`self.CameraRotation`))

(fn `UserConstructionScript`
  (`parent.UserConstructionScript`)
  (bind _asbp_detection (cast `/Game/Insider/Blueprints/Core/BP_Detection` (`ChildActorComponent.ChildActor` (`self.Detection`))))
  (bind _output_get (set `self.DetectionRef` _asbp_detection))
  (`/Game/Insider/Blueprints/Core/BP_Detection.SetBillboardTexture` _output_get (`self.DetectionSprite`)))