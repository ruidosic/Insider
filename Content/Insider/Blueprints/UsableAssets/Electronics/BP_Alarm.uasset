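; BP_Alarm is a usable electronic alarm with a mesh, light and 3D sound.
; While powered on and not alarmed, a delayed FlipFlop loop blinks the standby mesh and light.
; Alarm and Disalarm events switch the mesh, light visibility and intensity, start or stop the attached sound, and call GameEventCheck for the new state.
; The construction script creates game events and applies the initial off mesh and light settings.
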(event `self.ReceiveBeginPlay`
  ;[1 1 1] Begin Play
  (if (`self.On / Off`)
    (`self.RestoreOn`)))

(event `RestoreOn`
  ;[1 1 1] On / Off
  (`KismetSystemLibrary.Delay` (`self.Stand By Light Delay (Sec)`) :!label _label)
  (if (`self.Alarm On / Off`)
    _
    (elif (`self.On / Off`)
      (`/Engine/EditorBlueprintResources/StandardMacros.FlipFlop`
        (:`A`
          (`/Game/Insider/Blueprints/Core/BP_Functions.SetMesh` (`self.AlarmMesh`) (`self.AlarmStandBy`))
          (`SceneComponent.SetVisibility` (`self.AlarmLight`) true false)
          (goto _label))
        (:`B`
          (`/Game/Insider/Blueprints/Core/BP_Functions.SetMesh` (`self.AlarmMesh`) (`self.AlarmOff`))
          (`SceneComponent.SetVisibility` (`self.AlarmLight`) false false)
          (goto _label))))))

(event `self.Open/On`
  (params (GameEvent :type Boolean))
  ;[1 1 1] On / Off
  (if (not GameEvent)
    (set `self.On / Off` true)
    (goto _label)))

(event `self.Close/Off`
  (params (GameEvent :type Boolean))
  ;[1 1 1] On / Off
  (if (not GameEvent)
    (set `self.On / Off` false)
    (`/Game/Insider/Blueprints/Core/BP_Functions.SetMesh` (`self.AlarmMesh`) (`self.AlarmOff`))
    (`SceneComponent.SetVisibility` (`self.AlarmLight`) false false)))

(event `self.Alarm`
  (params (GameEvent :type Boolean))
  (bind _alarm_on___off (`self.Alarm On / Off`))
  (bind _alarmsound (`self.AlarmSound`))
  ;[1 1 1] Alarm / Disalarm
  (if (not GameEvent)
    (set `self.Alarm On / Off` true)
    (`/Game/Insider/Blueprints/Core/BPM_CoreEngine.GE_3DSound` _alarmsound false _alarmsound (`self.AlarmMesh`) (`self.Alarm Attenuation`))
    (`/Game/Insider/Blueprints/Core/BP_Functions.SetMesh` (`self.AlarmMesh`) (select `bool` _alarm_on___off :`false` (`self.AlarmOff`) :`true` (`self.AlarmOn`)) :!label _label_2)
    (`SceneComponent.SetVisibility` (`self.AlarmLight`) _alarm_on___off false)
    (`LightComponent.SetIntensity` (`self.AlarmLight`) (select `bool` (`self.Alarm On / Off`) :`false` (`self.Stand By Light Intensity`) :`true` (`self.Alarm Light Intensity`)))
    (`self.GameEventCheck` (select `bool` (`self.Alarm On / Off`) :`false` "NewEnumerator35" :`true` "NewEnumerator34" :!type "/Game/Insider/Blueprints/Events/Enums/Enum_GameEventCheck Enum"))))

(event `self.Disalarm`
  (params (GameEvent :type Boolean))
  ;[1 1 1] Alarm / Disalarm
  (if (not GameEvent)
    (set `self.Alarm On / Off` false)
    (`/Game/Insider/Blueprints/Core/BPM_CoreEngine.GE_Stop3DSound ` (`self.AlarmSound`))
    (goto _label_2)))

(fn `UserConstructionScript`
  (`parent.UserConstructionScript`)
  (set `self.GameEvents` (`self.CreateGameEvent`))
  (`/Game/Insider/Blueprints/Core/BP_Functions.SetMesh` (`self.AlarmMesh`) (`self.AlarmOff`))
  (`LightComponent.SetLightColor` (`self.AlarmLight`) (`self.AlarmLightColor`) true)
  (`LightComponent.SetIntensity` (`self.AlarmLight`) (`self.Stand By Light Intensity`)))