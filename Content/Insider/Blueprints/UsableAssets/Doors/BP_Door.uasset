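; Base door actor for interactive simple, controlled and sliding doors, with configurable meshes, async-loaded sounds and tag-selected settings.
; Use or an optional trigger overlap toggles open/close, leaving handle and door motion to child overrides.
; Alternative use locks or unlocks with a key, opening a key-filtered inventory if required, or knocks when locked without one.
; A reversible timeline animates the lock, updates state and fires game-event checks.
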(event `self.ReceiveBeginPlay`
  ;[1 1 1] Begin Play / Load Sound Async
  (`self.Load Sound Async`))

(event `Load Sound Async`
  ;[1 1 1] Assync Load Sounds
  (bind _sound (`/Game/Insider/Blueprints/Core/BPM_CoreEngine.SoundAsyncLoad` (`self.KnockKnock Sound`)))
  (set `self.KnockKnockSound` _sound)
  (bind _sound_2 (`/Game/Insider/Blueprints/Core/BPM_CoreEngine.SoundAsyncLoad` (`self.CloseHit Sound`)))
  (set `self.CloseHitSound` _sound_2)
  (bind _sound_3 (`/Game/Insider/Blueprints/Core/BPM_CoreEngine.SoundAsyncLoad` (`self.OpenHit Sound`)))
  (set `self.OpenHitSound` _sound_3)
  (bind _sound_4 (`/Game/Insider/Blueprints/Core/BPM_CoreEngine.SoundAsyncLoad` (`self.Creak Sound`)))
  (set `self.CreakSound` _sound_4)
  (bind _sound_5 (`/Game/Insider/Blueprints/Core/BPM_CoreEngine.SoundAsyncLoad` (`self.Lock Sound`)))
  (set `self.LockSound` _sound_5)
  (bind _sound_6 (`/Game/Insider/Blueprints/Core/BPM_CoreEngine.SoundAsyncLoad` (`self.Unlock Sound`)))
  (set `self.UnlockSound` _sound_6)
  (bind _sound_7 (`/Game/Insider/Blueprints/Core/BPM_CoreEngine.SoundAsyncLoad` (`self.Force Sound`)))
  (set `self.ForceSound` _sound_7)
  (bind _sound_8 (`/Game/Insider/Blueprints/Core/BPM_CoreEngine.SoundAsyncLoad` (`self.HandleOpen Sound`)))
  (set `self.HandleOpenSound` _sound_8)
  (bind _sound_9 (`/Game/Insider/Blueprints/Core/BPM_CoreEngine.SoundAsyncLoad` (`self.HandleRelease Sound`)))
  (set `self.HandleReleaseSound` _sound_9)
  (bind _sound_10 (`/Game/Insider/Blueprints/Core/BPM_CoreEngine.SoundAsyncLoad` (`self.DoorOpen Sound`)))
  (set `self.DoorOpenSound` _sound_10)
  (bind _sound_11 (`/Game/Insider/Blueprints/Core/BPM_CoreEngine.SoundAsyncLoad` (`self.DoorClose Sound`)))
  (set `self.DoorCloseSound` _sound_11)
  (bind _attenuation (`/Game/Insider/Blueprints/Core/BPM_CoreEngine.AttenuationAsyncLoad` (`self.Attenuation `)))
  (set `self.Attenuation` _attenuation))

(event `self.TriggerForUse.OnComponentBeginOverlap`
  (params (OverlappedComponent :type "PrimitiveComponent Object Reference") (OtherActor :type "Actor Object Reference") (OtherComp :type "PrimitiveComponent Object Reference") (OtherBodyIndex :type Integer) (bFromSweep :type Boolean) (SweepResult :type "HitResult Structure (by ref)"))
  ;[1 0 0.001607 1 20] Interaction
  ;;[1 1 1] Overlap With Player
  (if (and (== OtherActor (`GameplayStatics.GetPlayerPawn` 0)) (`self.UseTrigger`))
    (bind _as_core_engine (`/Game/Insider/Blueprints/Core/BP_Functions.GetPlayer`))
    (`/Game/Insider/Blueprints/Core/BP_CoreEngine.UseOverlappedActor` _as_core_engine self)))

(event `self.Use`
  (params (GameEvent :type Boolean))
  ;[1 0 0.001607 1 20] Interaction
  ;;[1 1 1 1 16] Use
  (`/Game/Insider/Blueprints/Core/BPM_CoreEngine.GE_CheckInteraction`)
  (if (`self.Open`)
    (`self.Close/Off` false)
    (else
      (`self.Open/On` false))))

(event `self.AlternativeUse`
  (params (GameEvent :type Boolean))
  ;[1 0 0.001607 1 20] Interaction
  ;;[1 1 1 1 20] Alternative Use
  (`/Game/Insider/Blueprints/Core/BPM_CoreEngine.GE_CheckInteraction`)
  (if (`self.HasLock`)
    (if (`self.AskForKey`)
      (if GameEvent
        (if (`self.PlayerHasKey`) :!label _label
          (if (`self.Locked`)
            (`self.Unlock` false)
            (else
              (`self.Lock` false)))
          (elif (`self.Locked`)
            (if (not (`self.Open`))
              (`self.KnockDoor`))))
        (else
          (`self.SelectKey` true)))
      (else
        (goto _label)))))

(event `LockDoor`
  ;[1 1 1] Lock / Unlock
  (`/Game/Insider/Blueprints/Core/BPM_CoreEngine.GE_3DSound` null false (`self.LockSound`) (`self.LockPivot`) (`self.Attenuation`))
  (bind (_direction _animation) (`Timeline|LockTimeline` :!via `PlayFromStart` :!label _label_2)
    (:`Update`
      (`SceneComponent.K2_SetRelativeRotation` (`self.LockPivot`) (`KismetMathLibrary.RLerp` (`self.UnlockRotation`) (`self.LockRotation`) _animation) false false))
    (:`Finished`
      (switch `ETimelineDirection` _direction
        (:`Forward`
          (set `self.Locked` true)
          (`self.GameEventCheck` "NewEnumerator8")
          (set `self.InteractionEnabled` true))
        (:`Backward`
          (set `self.Locked` false)
          (`self.GameEventCheck` "NewEnumerator9")
          (set `self.InteractionEnabled` true)
          (bind _as_core_engine (`/Game/Insider/Blueprints/Core/BP_Functions.GetPlayer`))
          (bind _filteredarray (`KismetArrayLibrary.FilterArray` (`/Game/Insider/Blueprints/Core/BP_CoreEngine.PlayerInventory` _as_core_engine) "/Game/Insider/Blueprints/UsableAssets/Inventory/Keys/BP_Key.BP_Key_C"))
          (for _array_element _filteredarray
            (bind _asbp_key (cast `/Game/Insider/Blueprints/UsableAssets/Inventory/Keys/BP_Key` _array_element))
            (`/Game/Insider/Blueprints/UsableAssets/Inventory/Keys/BP_Key.CheckUnlocked` _asbp_key)))))))

(event `self.Lock`
  (params (GameEvent :type Boolean))
  ;[1 0.9226 0.02852] (Overriden parent functions)
  ;;[1 1 1] Lock / Unlock
  (`/Game/Insider/Blueprints/Core/BPM_CoreEngine.GE_CheckInteraction`)
  (if (`self.HasLock`)
    (if (not (`self.Locked`))
      (set `self.InteractionEnabled` false)
      (if (`self.Open`)
        (`self.CloseDoor` true)
        (else
          (`self.LockDoor`))))))

(event `self.Open/On`
  (params (GameEvent :type Boolean))
  ;[1 0.9226 0.02852] (Overriden parent functions)
  ;;[1 1 1] Open / Close
  (`/Game/Insider/Blueprints/Core/BPM_CoreEngine.GE_CheckInteraction`)
  (if (`self.Open`)
    (`self.ToggleDoor` :!label _label_3)
    (else
      (`self.OpenHandle`))))

(event `OpenHandle`
  ;[0.4596 1 0.4362] Handle Settings
  ;;[1 1 1] Function To Override In  Children
)

(event `UnlockDoor`
  ;[1 1 1] Lock / Unlock
  (`/Game/Insider/Blueprints/Core/BPM_CoreEngine.GE_3DSound` null false (`self.UnlockSound`) (`self.LockPivot`) (`self.Attenuation`))
  (goto _label_2 :!via `ReverseFromEnd`))

(event `self.Close/Off`
  (params (GameEvent :type Boolean))
  ;[1 0.9226 0.02852] (Overriden parent functions)
  ;;[1 1 1] Open / Close
  (`/Game/Insider/Blueprints/Core/BPM_CoreEngine.GE_CheckInteraction`)
  (if (`self.Open`)
    (goto _label_3)))

(event `ResetHandle`
  ;[0.4596 1 0.4362] Handle Settings
  ;;[1 1 1] Function To Override In  Children
)

(event `self.Unlock`
  (params (GameEvent :type Boolean))
  ;[1 0.9226 0.02852] (Overriden parent functions)
  ;;[1 1 1] Lock / Unlock
  (`/Game/Insider/Blueprints/Core/BPM_CoreEngine.GE_CheckInteraction`)
  (if (`self.HasLock`)
    (if (`self.Locked`)
      (set `self.InteractionEnabled` false)
      (`self.UnlockDoor`))))

(event `KnockDoor`
  ;[0 0.2313 0.8927 1 20] Door Settings
  ;;[1 1 1 1 16] Knock Door
  (if (not (`KismetSystemLibrary.IsValid` (stale _returnvalue)))
    (bind _returnvalue (`GameplayStatics.SpawnSoundAttached` (`self.KnockKnockSound`) (`self.LockPivot`) "None" (0.0 0.0 0.0) (struct) "KeepRelativeOffset" false 1.0 1.0 0.0 null null))
    (`self.GameEventCheck` "NewEnumerator10")))

(event `ToggleDoor`
  ;[0 0.2313 0.8927 1 20] Door Settings
  ;;[1 1 1] Function To Override In  Children
)

(event `SelectKey`
  (params (`Open Inventory` :type Boolean))
  ;[0 0 0] Key Settings
  ;;[1 1 1 1 20] Select Key
  (bind _as_core_engine (`/Game/Insider/Blueprints/Core/BP_Functions.GetPlayer`))
  (if (`/Game/Insider/Blueprints/Core/BP_CoreEngine.FilterInventory` _as_core_engine)
    (bind _filteredarray (`KismetArrayLibrary.FilterArray` (`/Game/Insider/Blueprints/Core/BP_CoreEngine.PlayerInventory` _as_core_engine) "/Game/Insider/Blueprints/UsableAssets/Inventory/Keys/BP_Key.BP_Key_C"))
    (if (> (`KismetArrayLibrary.Array_Length` _filteredarray) 0)
      (set `/Game/Insider/Blueprints/Core/BP_CoreEngine.InventoryFilter` "NewEnumerator2" _as_core_engine)
      (set `/Game/Insider/Blueprints/Core/BP_CoreEngine.UsableRef` self _as_core_engine)
      (`/Game/Insider/Blueprints/Core/BP_Functions.SetFilteredItems` "/Game/Insider/Blueprints/UsableAssets/Inventory/Keys/BP_Key.BP_Key_C" true true (select `bool` (`self.Locked`) :`false` "Unlock" :`true` "Lock" :!type "Text"))
      (if `Open Inventory`
        (`/Game/Insider/Blueprints/Core/BP_Functions.OpenInventory`))
      (else
        (`/Game/Insider/Blueprints/Core/BP_Functions.Notice` "There is no any" "Key" "in inventory")))))

(event `OpenDoor`
  ;[0 0.2313 0.8927 1 20] Door Settings
  ;;[1 1 1] Function To Override In  Children
)

(event `CloseDoor`
  (params (Lock :type Boolean))
  ;[0 0.2313 0.8927 1 20] Door Settings
  ;;[1 1 1] Function To Override In  Children
)

(event `ForceDoor`
  ;[0 0.2313 0.8927 1 20] Door Settings
  ;;[1 1 1] Function To Override In  Children
)

(event `self.TakeKey`
  (params (GameEvent :type Boolean))
  ;[0 0 0] Key Settings
  ;;[1 1 1] Take key (Overriden parent's)
  (set `self.PlayerHasKey` true))

(fn `SetInitialConfiguration`
  ;[1 1 1] Starter Settings
  (if (`self.Open`)
    (set `self.Locked` false))
  (`SceneComponent.K2_SetRelativeRotation` (`self.LockPivot`) (select `bool` (`self.Locked`) :`false` (`self.UnlockRotation`) :`true` (`self.LockRotation`)) false false)
  (if (not (`self.HasLock`))
    (set `self.Locked` false)))

(fn `SetMeshesAndMaterials`
  (`/Game/Insider/Blueprints/Core/BP_Functions.SetMesh` (`self.Door`) (`self.DoorMesh`))
  (`/Game/Insider/Blueprints/Core/BP_Functions.SetMesh` (`self.DoorFrame`) (`self.DoorFrameMesh`))
  (`/Game/Insider/Blueprints/Core/BP_Functions.SetMesh` (`self.HandleBaseFront`) (`self.HandleBaseFrontMesh`))
  (`/Game/Insider/Blueprints/Core/BP_Functions.SetMesh` (`self.HandleBaseBack`) (`self.HandleBaseBackMesh`))
  (`/Game/Insider/Blueprints/Core/BP_Functions.SetMesh` (`self.HandleFront`) (`self.HandleFrontMesh`))
  (`/Game/Insider/Blueprints/Core/BP_Functions.SetMesh` (`self.HandleBack`) (`self.HandleBackMesh`))
  (`/Game/Insider/Blueprints/Core/BP_Functions.SetMesh` (`self.LockFront`) (`self.LockFrontMesh`))
  (`/Game/Insider/Blueprints/Core/BP_Functions.SetMesh` (`self.LockBack`) (`self.LockBackMesh`)))

(fn `SetMeshesVisibilityAndCollision`
  (bind _hasframe (`self.HasFrame`))
  (bind _hashandlebase (`self.HasHandleBase`))
  (bind _hashandle (`self.HasHandle`))
  ;[1 1 1] Active / Disactive different Part of Door
  (`SceneComponent.SetVisibility` (`self.DoorFrame`) _hasframe false)
  (`PrimitiveComponent.SetCollisionEnabled` (`self.DoorFrame`) (select `bool` _hasframe :`false` "NoCollision" :`true` "QueryAndPhysics" :!type "ECollisionEnabled Enum"))
  (`SceneComponent.SetVisibility` (`self.HandleBack`) _hashandle false)
  (`SceneComponent.SetVisibility` (`self.HandleFront`) _hashandle false)
  (`PrimitiveComponent.SetCollisionEnabled` (`self.HandleBack`) (select `bool` _hashandle :`false` "NoCollision" :`true` "QueryAndPhysics" :!type "ECollisionEnabled Enum"))
  (`PrimitiveComponent.SetCollisionEnabled` (`self.HandleFront`) (select `bool` _hashandle :`false` "NoCollision" :`true` "QueryAndPhysics" :!type "ECollisionEnabled Enum"))
  (`SceneComponent.SetVisibility` (`self.HandleBaseBack`) _hashandlebase false)
  (`SceneComponent.SetVisibility` (`self.HandleBaseFront`) _hashandlebase false)
  (`PrimitiveComponent.SetCollisionEnabled` (`self.HandleBaseBack`) (select `bool` _hashandlebase :`false` "NoCollision" :`true` "QueryAndPhysics" :!type "ECollisionEnabled Enum"))
  (`PrimitiveComponent.SetCollisionEnabled` (`self.HandleBaseFront`) (select `bool` _hashandlebase :`false` "NoCollision" :`true` "QueryAndPhysics" :!type "ECollisionEnabled Enum")))

(fn `SetTimelinesPlayRate`
  ;[1 1 1] At now this function consist only one Timeline Play Rate for Lock Anim
  (`/Game/Insider/Blueprints/Core/BP_Functions.PlayRate` (`self.LockTimeline`) (`self.Lock / Unlock Duration (Sec)`)))

(fn `SetupSettings`
  (params (`Game Events` :type "Array of /Game/Insider/Blueprints/Events/Structs/Struct_GameEvents Structure") (TriggerSettings :type "/Game/Insider/Blueprints/UsableAssets/Doors/Structs/Struct_TriggerSettings Structure") (MeshSettings :type "/Game/Insider/Blueprints/UsableAssets/Doors/Structs/Struct_DoorMeshSettings Structure") (SimpleDoorSettings :type "/Game/Insider/Blueprints/UsableAssets/Doors/Structs/Struct_DoorSettings Structure") (ControlledDoorSettings :type "/Game/Insider/Blueprints/UsableAssets/Doors/Structs/ControlledDoor/Struct_CD_Settings Structure") (SlidingDoorSettings :type "/Game/Insider/Blueprints/UsableAssets/Doors/Structs/SlidingDoor/Struct_SlidingDoorSettings Structure") (Attenuation :type "SoundAttenuation Soft Object Reference"))
  (bind (_hasframe _haslock _hashandlebase _hashandle _doormesh _doorframemesh _handlebasefrontmesh _handlebasebackmesh _handlefrontmesh _handlebackmesh _lockfrontmesh _lockbackmesh) (break `/Game/Insider/Blueprints/UsableAssets/Doors/Structs/Struct_DoorMeshSettings` (`self.MeshSettings`)))
  (bind (_usetrigger _triggersize) (break `/Game/Insider/Blueprints/UsableAssets/Doors/Structs/Struct_TriggerSettings` (`self.TriggerSettings`)))
  (bind (_doorinfo _handleinfo _lockinfo _forceinfo _keyinfo) (break `/Game/Insider/Blueprints/UsableAssets/Doors/Structs/Struct_DoorSettings` (`self.SimpleDoorSettings`)))
  (bind (_doorname _openlocation _closelocation _openclosedurationsec _opensound _closesound _openhitsound _closehitsound) (break `/Game/Insider/Blueprints/UsableAssets/Doors/Structs/ControlledDoor/Struct_CD_Settings` (`self.ControlledDoorSetting`)))
  (bind (_doorinfo_2 _handleinfo_2 _lockinfo_2 _forceinfo_2 _keyinfo_2) (break `/Game/Insider/Blueprints/UsableAssets/Doors/Structs/SlidingDoor/Struct_SlidingDoorSettings` (`self.SlidingDoorSettings`)))
  (bind ((`DoorName_3_C9CF160A42B917004D7930A187B43B8D` _doorname_2) (`Open_6_E28633294836B9101746FA9B75DCE4FC` _open) (`DoorOpenCloseDurationSec_9_2B651E6746FA9A96987DC5BCDD9DCC8B` _dooropenclosedurationsec) (`DoorOpenRotation_15_54D234E24ACE84C9F0A30C868B8A4A47` _dooropenrotation) (`DoorCloseRotation_17_F636C2174DEEA7DC5C7351916696F8F2` _doorcloserotation) (`CloseHitSound_25_653A4D7E44AFFD10CFC66F973D04AE0D` _closehitsound_2) (`CreakSound_26_8B65A7D84C0DBFCAB3D8D5AE066C5FD3` _creaksound)) (break `/Game/Insider/Blueprints/UsableAssets/Doors/Structs/Struct_DoorInfo` _doorinfo))
  (bind (_handleopenreleasedurationsec _handleopenrotation _handlereleaserotation _handleopensound _handlereleasesound) (break `/Game/Insider/Blueprints/UsableAssets/Doors/Structs/Struct_DoorHandleInfo` _handleinfo))
  (bind (_lockunlockdurationsec _locked _locksound _unlocksound _lockrotation _unlockrotation) (break `/Game/Insider/Blueprints/UsableAssets/Doors/Structs/Struct_DoorLockInfo` _lockinfo))
  (bind (_forcedurationsec _forcerotation _forcesound) (break `/Game/Insider/Blueprints/UsableAssets/Doors/Structs/Struct_DoorForceInfo` _forceinfo))
  (bind (_askforkey _playerhaskey) (break `/Game/Insider/Blueprints/UsableAssets/Doors/Structs/Struct_DoorKeyInfo` _keyinfo))
  (bind (_doorname_3 _open_2 _dooropenclosedurationsec_2 _knockknocksound _dooropenlocation _doorcloselocation _closehitsound_3 _creaksound_2 _dooropensound _doorclosesound) (break `/Game/Insider/Blueprints/UsableAssets/Doors/Structs/SlidingDoor/Struct_SlidingDoorInfo` _doorinfo_2))
  (bind (_handleopenreleasedurationsec_2 _handleopenrotation_2 _handlereleaserotation_2 _handleopensound_2 _handlereleasesound_2) (break `/Game/Insider/Blueprints/UsableAssets/Doors/Structs/Struct_DoorHandleInfo` _handleinfo_2))
  (bind (_lockunlockdurationsec_2 _locked_2 _locksound_2 _unlocksound_2 _lockrotation_2 _unlockrotation_2) (break `/Game/Insider/Blueprints/UsableAssets/Doors/Structs/Struct_DoorLockInfo` _lockinfo_2))
  (bind (_forcedurationsec_2 _forcerotation_2 _forcesound_2) (break `/Game/Insider/Blueprints/UsableAssets/Doors/Structs/Struct_DoorForceInfo` _forceinfo_2))
  (bind (_askforkey_2 _playerhaskey_2) (break `/Game/Insider/Blueprints/UsableAssets/Doors/Structs/Struct_DoorKeyInfo` _keyinfo_2))
  ;[1 1 1] Setup Initial Defaults
  (set `self.GameEvents` `Game Events`)
  (set `self.TriggerSettings` TriggerSettings)
  (set `self.MeshSettings` MeshSettings)
  (set `self.SimpleDoorSettings` SimpleDoorSettings)
  (set `self.ControlledDoorSetting` ControlledDoorSettings)
  (set `self.SlidingDoorSettings` SlidingDoorSettings)
  ;[1 1 1] Setup Attenuation
  (set `self.Attenuation ` Attenuation)
  ;[1 1 1] Setup Trigger Settings
  (set `self.UseTrigger` _usetrigger)
  (set `self.TriggerSize` _triggersize)
  ;[1 1 1] Setup Mesh Settings
  (set `self.HasFrame` _hasframe)
  (set `self.HasLock` _haslock)
  (set `self.HasHandleBase` _hashandlebase)
  (set `self.HasHandle` _hashandle)
  (set `self.DoorMesh` _doormesh)
  (set `self.DoorFrameMesh` _doorframemesh)
  (set `self.HandleBaseFrontMesh` _handlebasefrontmesh)
  (set `self.HandleBaseBackMesh` _handlebasebackmesh)
  (set `self.HandleFrontMesh` _handlefrontmesh)
  (set `self.HandleBackMesh` _handlebackmesh)
  (set `self.LockFrontMesh` _lockfrontmesh)
  (set `self.LockBackMesh` _lockbackmesh)
  ;[1 1 1] Setup Doors Settings
  ;;[1 0 0] Check Door
  (`self.CheckTag`
    (:`SimpleDoor`
      (set `self.DoorName` _doorname_2)
      (set `self.Open` _open)
      (set `self.Door Open / Close Duration (Sec)` _dooropenclosedurationsec)
      (set `self.DoorOpenRotation` _dooropenrotation)
      (set `self.DoorCloseRotation` _doorcloserotation)
      (set `self.CloseHit Sound` _closehitsound_2)
      (set `self.Creak Sound` _creaksound)
      (set `self.Handle Open / Release Duration (Sec)` _handleopenreleasedurationsec)
      (set `self.HandleOpenRotation` _handleopenrotation)
      (set `self.HandleReleaseRotation` _handlereleaserotation)
      (set `self.HandleOpen Sound` _handleopensound)
      (set `self.HandleRelease Sound` _handlereleasesound)
      (set `self.Lock / Unlock Duration (Sec)` _lockunlockdurationsec)
      (set `self.Locked` _locked)
      (set `self.Lock Sound` _locksound)
      (set `self.Unlock Sound` _unlocksound)
      (set `self.LockRotation` _lockrotation)
      (set `self.UnlockRotation` _unlockrotation)
      (set `self.ForceDuration (Sec)` _forcedurationsec)
      (set `self.ForceRotation` _forcerotation)
      (set `self.Force Sound` _forcesound)
      (set `self.AskForKey` _askforkey)
      (set `self.PlayerHasKey` _playerhaskey))
    (:`ControlledDoor`
      (set `self.DoorName` _doorname)
      (set `self.OpenLocation` _openlocation)
      (set `self.CloseLocation` _closelocation)
      (set `self.Door Open / Close Duration (Sec)` _openclosedurationsec)
      (set `self.DoorOpen Sound` _opensound)
      (set `self.DoorClose Sound` _closesound)
      (set `self.OpenHit Sound` _openhitsound)
      (set `self.CloseHit Sound` _closehitsound))
    (:`SlidingDoor`
      (set `self.DoorName` _doorname_3)
      (set `self.Open` _open_2)
      (set `self.Door Open / Close Duration (Sec)` _dooropenclosedurationsec_2)
      (set `self.OpenLocation` _dooropenlocation)
      (set `self.CloseLocation` _doorcloselocation)
      (set `self.CloseHit Sound` _closehitsound_3)
      (set `self.Creak Sound` _creaksound_2)
      (set `self.DoorOpen Sound` _dooropensound)
      (set `self.DoorClose Sound` _doorclosesound)
      (set `self.Handle Open / Release Duration (Sec)` _handleopenreleasedurationsec_2)
      (set `self.HandleOpenRotation` _handleopenrotation_2)
      (set `self.HandleReleaseRotation` _handlereleaserotation_2)
      (set `self.HandleOpen Sound` _handleopensound_2)
      (set `self.HandleRelease Sound` _handlereleasesound_2)
      (set `self.Lock / Unlock Duration (Sec)` _lockunlockdurationsec_2)
      (set `self.Locked` _locked_2)
      (set `self.Lock Sound` _locksound_2)
      (set `self.Unlock Sound` _unlocksound_2)
      (set `self.LockRotation` _lockrotation_2)
      (set `self.UnlockRotation` _unlockrotation_2)
      (set `self.ForceDuration (Sec)` _forcedurationsec_2)
      (set `self.ForceRotation` _forcerotation_2)
      (set `self.Force Sound` _forcesound_2)
      (set `self.AskForKey` _askforkey_2)
      (set `self.PlayerHasKey` _playerhaskey_2))))

(fn `SetUseTriggerSettings`
  (bind _triggerforuse (`self.TriggerForUse`))
  (bind _triggersize (`self.TriggerSize`))
  (`BoxComponent.SetBoxExtent` _triggerforuse _triggersize true)
  (`SceneComponent.K2_SetRelativeLocation` _triggerforuse _triggersize false false))

(fn `UserConstructionScript`
  (`self.SetMeshesAndMaterials`)
  (`self.SetMeshesVisibilityAndCollision`)
  (`self.SetTimelinesPlayRate`)
  (`self.SetUseTriggerSettings`)
  (`self.SetInitialConfiguration`))