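; BP_SimpleDoor is a usable hinged door that rotates open and closed, or jolts when forced while locked.
; It overrides parent setup events, with construction-time settings and duration-based timeline play rates.
; A handle timeline triggers either opening or forcing, while the open/close timeline also reverses for closing.
; Timeline event tracks drive sounds, state updates, game events and optional locking after closing.
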(event `self.SetInitialConfiguration`
  ;[1 0 0] Override Parent Setup Functions
  ;;[1 1 1] InitialConfiguration
  (`TimelineComponent.SetNewTime` (`self.OpenCloseTimeline`) (select `bool` (`self.Open`) :`true` 1.0 :!type "Float (single-precision)"))
  (`SceneComponent.K2_SetRelativeRotation` (`self.Door`) (select `bool` (`self.Open`) :`false` (`self.DoorCloseRotation`) :`true` (`self.DoorOpenRotation`)) false false)
  (`parent.SetInitialConfiguration`))

(event `self.SetTimelinesPlayRate`
  ;[1 0 0] Override Parent Setup Functions
  ;;[1 1 1] Set Timelines Play Rate
  (`parent.SetTimelinesPlayRate`)
  (`/Game/Insider/Blueprints/Core/BP_Functions.PlayRate` (`self.OpenCloseTimeline`) (`self.Door Open / Close Duration (Sec)`))
  (`/Game/Insider/Blueprints/Core/BP_Functions.PlayRate` (`self.ForceTimeline`) (`self.ForceDuration (Sec)`))
  (`/Game/Insider/Blueprints/Core/BP_Functions.PlayRate` (`self.HandleTimeline`) (`self.Handle Open / Release Duration (Sec)`)))

(event `self.OpenHandle`
  ;[1 1 1] Handle Settings
  (bind (_direction _animation) (`Timeline|HandleTimeline` :!label _label)
    (:`Update`
      (`SceneComponent.K2_SetRelativeRotation` (`self.HandlePivot`) (`KismetMathLibrary.RLerp` (`self.HandleReleaseRotation`) (`self.HandleOpenRotation`) _animation) false false))
    (:`HandleOpenSound`
      (`/Game/Insider/Blueprints/Core/BPM_CoreEngine.GE_3DSound` null false (`self.HandleOpenSound`) (`self.HandlePivot`) (`self.Attenuation`)))
    (:`HandleReleaseSound`
      (`/Game/Insider/Blueprints/Core/BPM_CoreEngine.GE_3DSound` null false (`self.HandleReleaseSound`) (`self.HandlePivot`) (`self.Attenuation`)))
    (:`OpenDoor`
      (if (`self.Locked`)
        (`self.ForceDoor`)
        (else
          (`self.OpenDoor`))))))

(event `self.ResetHandle`
  ;[1 1 1] Handle Settings
  (goto _label :!via `SetNewTime`))

(event `self.ForceDoor`
  (bind _forcesound (`self.ForceSound`))
  ;[1 1 1] Force Open
  (bind (_direction _animation) (`Timeline|ForceTimeline` :!via `PlayFromStart`)
    (:`Update`
      (`SceneComponent.K2_SetRelativeRotation` (`self.Door`) (`KismetMathLibrary.RLerp` (`self.DoorCloseRotation`) (`self.ForceRotation`) _animation) false false))
    (:`Finished`
      (`self.ResetHandle`)
      (`self.GameEventCheck` "NewEnumerator11"))
    (:`ForceSound`
      (`/Game/Insider/Blueprints/Core/BPM_CoreEngine.GE_3DSound` _forcesound false _forcesound (`self.HandlePivot`) (`self.Attenuation`)))))

(event `self.ToggleDoor`
  ;[1 1 1 1 16] Toggle Door
  (switch `ETimelineDirection` (stale `self.OpenDoor` _direction)
    (:`Forward`
      (`self.CloseDoor` false))
    (:`Backward`
      (`self.OpenDoor`))))

(event `self.OpenDoor`
  (bind _creaksound (`self.CreakSound`))
  ;[1 1 1 1 16] Open / Close Door
  (bind (_direction _animation) (`Timeline|OpenCloseTimeline` :!label _label_2)
    (:`Update`
      (`SceneComponent.K2_SetRelativeRotation` (`self.Door`) (`KismetMathLibrary.RLerp` (`self.DoorCloseRotation`) (`self.DoorOpenRotation`) _animation) true true))
    (:`Finished`
      (`/Game/Insider/Blueprints/Core/BPM_CoreEngine.GE_Stop3DSound ` (`self.CreakSound`)))
    (:`OpenCloseCheck`
      (switch `ETimelineDirection` _direction
        (:`Forward`
          (set `self.Open` true)
          (`self.GameEventCheck` "NewEnumerator1"))
        (:`Backward`
          (set `self.Open` false)
          (`/Game/Insider/Blueprints/Core/BPM_CoreEngine.GE_3DSound` null false (`self.CloseHitSound`) (`self.HandlePivot`) (`self.Attenuation`))
          (`self.ResetHandle`)
          (`self.GameEventCheck` "NewEnumerator2")
          (if (stale `self.CloseDoor` Lock)
            (`self.LockDoor`)))))
    (:`CreakSound`
      (`/Game/Insider/Blueprints/Core/BPM_CoreEngine.GE_3DSound` _creaksound false _creaksound (`self.Door`) (`self.Attenuation`)))))

(event `self.CloseDoor`
  (params (Lock :type Boolean))
  ;[1 1 1 1 16] Open / Close Door
  (goto _label_2 :!via `Reverse`))

(fn `UserConstructionScript`
  (`self.SetupSettings` (`self.CreateGameEvents`) (`self.Trigger Settings`) (`self.Mesh Settings`) (`self.DoorSettings`) (struct) (struct) (`self.SoundAttenuation`))
  (`parent.UserConstructionScript`))