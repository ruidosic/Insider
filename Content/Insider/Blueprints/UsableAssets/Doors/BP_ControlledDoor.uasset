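; BP_ControlledDoor is a usable, lockless door that slides between closed and open locations.
; A timeline lerps the DoorPivot location, with open, close and hit sounds attached to the pivot.
; A timeline event updates the Open state and fires game event checks by direction, while toggling reverses the current direction.
; It overrides parent setup functions to snap to its initial state and set play rate from duration.
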(event `self.SetInitialConfiguration`
  ;[1 0 0] Override Parent Setup Functions
  (`self.RefreshDoor`))

(event `self.SetTimelinesPlayRate`
  ;[1 0 0] Override Parent Setup Functions
  (`/Game/Insider/Blueprints/Core/BP_Functions.PlayRate` (`self.OpenCloseTimeline`) (`self.Door Open / Close Duration (Sec)`)))

(event `self.Open/On`
  (params (GameEvent :type Boolean))
  ;[1 1 1] Open On / Open / Close / Toggle Door
  (`/Game/Insider/Blueprints/Core/BPM_CoreEngine.GE_CheckInteraction`)
  (if (`self.Open`)
    (`self.ToggleDoor`)
    (else
      (`self.OpenDoor`))))

(event `self.ToggleDoor`
  ;[1 1 1] Open On / Open / Close / Toggle Door
  (switch `ETimelineDirection` (stale `self.OpenDoor` _direction)
    (:`Forward`
      (`self.CloseDoor` false))
    (:`Backward`
      (`self.OpenDoor`))))

(event `self.OpenDoor`
  ;[1 1 1] Open On / Open / Close / Toggle Door
  (set `self.Opening` true)
  (`/Game/Insider/Blueprints/Core/BPM_CoreEngine.GE_3DSound` (`self.DoorCloseSound`) false (`self.DoorOpenSound`) (`self.DoorPivot`) (`self.Attenuation`))
  (bind (_direction _animation) (`Timeline|OpenCloseTimeline` :!label _label)
    (:`Update`
      (`SceneComponent.K2_SetRelativeLocation` (`self.DoorPivot`) (`KismetMathLibrary.VLerp` (`self.CloseLocation`) (`self.OpenLocation`) _animation) false false))
    (:`Finished`
      (switch `ETimelineDirection` _direction
        (:`Forward`
          (`/Game/Insider/Blueprints/Core/BPM_CoreEngine.GE_3DSound` (`self.DoorOpenSound`) false (`self.OpenHitSound`) (`self.DoorPivot`) (`self.Attenuation`)))))
    (:`OpenCloseCheck`
      (switch `ETimelineDirection` _direction
        (:`Forward`
          (set `self.Open` true)
          (`self.GameEventCheck` "NewEnumerator1"))
        (:`Backward`
          (set `self.Open` false)
          (`self.GameEventCheck` "NewEnumerator2")
          (`/Game/Insider/Blueprints/Core/BPM_CoreEngine.GE_3DSound` (`self.DoorCloseSound`) false (`self.CloseHitSound`) (`self.DoorPivot`) (`self.Attenuation`)))))))

(event `self.CloseDoor`
  (params (Lock :type Boolean))
  ;[1 1 1] Open On / Open / Close / Toggle Door
  (set `self.Opening` false)
  (`/Game/Insider/Blueprints/Core/BPM_CoreEngine.GE_3DSound` (`self.DoorOpenSound`) false (`self.DoorCloseSound`) (`self.DoorPivot`) (`self.Attenuation`))
  (goto _label :!via `Reverse`))

(event `self.AlternativeUse`
  (params (GameEvent :type Boolean))
  ;[1 1 1] Alternative Use Stub
)

(fn `RefreshDoor`
  (`TimelineComponent.SetNewTime` (`self.OpenCloseTimeline`) (select `bool` (`self.Open`) :`true` 1.0 :!type "Float (single-precision)"))
  (`SceneComponent.K2_SetRelativeLocation` (`self.DoorPivot`) (select `bool` (`self.Open`) :`false` (`self.CloseLocation`) :`true` (`self.OpenLocation`)) false false))

(fn `UserConstructionScript`
  (`self.SetupSettings` (`self.CreateGameEvents`) (`self.Trigger Settings`) (make `/Game/Insider/Blueprints/UsableAssets/Doors/Structs/Struct_DoorMeshSettings` true false false false (`self.Door Mesh`) (`self.Frame Mesh`)) (struct) (`self.Door Settings`) (struct) (`self.Sound Attenuation`))
  (`parent.UserConstructionScript`))