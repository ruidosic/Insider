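; Sliding door usable that overrides its parent's door logic to slide a pivot between closed and open locations.
; Interaction turns the handle, then opens the door, plays a forced-handle animation if locked, or toggles it if already open.
; Open/close, handle and force timelines drive lerped transforms, 3D sounds and game-event checks; closing resets the handle and can lock.
; Construction applies settings and initial pose, attaching the lock to the handle pivot.
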(event `self.SetInitialConfiguration`
  ;[1 0 0] Override Parent Setup Functions
  ;;[1 1 1] Set Initial Setup Timeline
  (`TimelineComponent.SetNewTime` (`self.OpenCloseTimeline`) (`self.Door Open / Close Duration (Sec)`))
  (`SceneComponent.K2_SetRelativeLocation` (`self.DoorPivot`) (select `bool` (`self.Open`) :`false` (`self.CloseLocation`) :`true` (`self.OpenLocation`)) false false)
  (`parent.SetInitialConfiguration`))

(event `self.SetTimelinesPlayRate`
  ;[1 0 0] Override Parent Setup Functions
  ;;[1 1 1] Set Timeline Play Rate
  (`parent.SetTimelinesPlayRate`)
  (`/Game/Insider/Blueprints/Core/BP_Functions.PlayRate` (`self.ForceTimeline`) (`self.ForceDuration (Sec)`))
  (`/Game/Insider/Blueprints/Core/BP_Functions.PlayRate` (`self.HandleTimeline`) (`self.Handle Open / Release Duration (Sec)`))
  (`/Game/Insider/Blueprints/Core/BP_Functions.PlayRate` (`self.OpenCloseTimeline`) (`self.Door Open / Close Duration (Sec)`)))

(event `self.ToggleDoor`
  ;[1 1 1] Toggle / Open / Close Door
  (switch `ETimelineDirection` (stale `self.OpenDoor` _direction)
    (:`Forward`
      (`self.CloseDoor` false))
    (:`Backward`
      (`self.OpenDoor`))))

(event `self.OpenDoor`
  ;[1 1 1] Toggle / Open / Close Door
  (`/Game/Insider/Blueprints/Core/BPM_CoreEngine.GE_3DSound` (`self.DoorCloseSound`) false (`self.DoorOpenSound`) (`self.HandlePivot`) (`self.Attenuation`))
  (bind (_direction _animation) (`Timeline|OpenCloseTimeline` :!label _label)
    (:`Update`
      (`SceneComponent.K2_SetRelativeLocation` (`self.DoorPivot`) (`KismetMathLibrary.VLerp` (`self.CloseLocation`) (`self.OpenLocation`) _animation) false false))
    (:`Finished`
      (`/Game/Insider/Blueprints/Core/BPM_CoreEngine.GE_Stop3DSound ` null)
      (`/Game/Insider/Blueprints/Core/BPM_CoreEngine.GE_Stop3DSound ` null))
    (:`OpenCloseCheck`
      (switch `ETimelineDirection` _direction
        (:`Forward`
          (set `self.Open` true)
          (`self.GameEventCheck` "NewEnumerator1"))
        (:`Backward`
          (set `self.Open` false)
          (`/Game/Insider/Blueprints/Core/BPM_CoreEngine.GE_3DSound` null false (`self.CloseHitSound`) (`self.HandlePivot`) (`self.Attenuation`))
          (`self.ResetHandle`)
          (`self.GameEventCheck` "NewEnumerator2")
          (if (stale `self.CloseDoor` Lock)
            (`self.LockDoor`)))))))

(event `self.CloseDoor`
  (params (Lock :type Boolean))
  ;[1 1 1] Toggle / Open / Close Door
  (`/Game/Insider/Blueprints/Core/BPM_CoreEngine.GE_3DSound` (`self.DoorOpenSound`) false (`self.DoorCloseSound`) (`self.HandlePivot`) (`self.Attenuation`))
  (goto _label :!via `Reverse`))

(event `self.OpenHandle`
  ;[1 1 1] Handle Settings
  (bind (_direction _animation) (`Timeline|HandleTimeline` :!label _label_2)
    (:`Update`
      (`SceneComponent.K2_SetRelativeRotation` (`self.HandlePivot`) (`KismetMathLibrary.RLerp` (`self.HandleReleaseRotation`) (`self.HandleOpenRotation`) _animation) false false))
    (:`Finished`
      (switch `ETimelineDirection` _direction
        (:`Forward`
          (if (`self.Locked`)
            (`self.ForceDoor`)
            (else
              (`self.OpenDoor`))))))
    (:`HandleOpenSound`
      (`/Game/Insider/Blueprints/Core/BPM_CoreEngine.GE_3DSound` null false (`self.HandleOpenSound`) (`self.HandlePivot`) (`self.Attenuation`)))
    (:`HandleReleaseSound`
      (`/Game/Insider/Blueprints/Core/BPM_CoreEngine.GE_3DSound` null false (`self.HandleReleaseSound`) (`self.HandlePivot`) (`self.Attenuation`)))))

(event `self.ResetHandle`
  ;[1 1 1] Handle Settings
  (goto _label_2 :!via `ReverseFromEnd`))

(event `self.ForceDoor`
  (bind _handleopensound (`self.HandleOpenSound`))
  ;[1 1 1] Force Settings
  (bind (_direction _animation) (`Timeline|ForceTimeline` :!via `PlayFromStart`)
    (:`Update`
      (`SceneComponent.K2_SetRelativeRotation` (`self.HandlePivot`) (`KismetMathLibrary.RLerp` (`self.HandleReleaseRotation`) (`self.ForceRotation`) _animation) false false)
      (`self.GameEventCheck` "NewEnumerator11"))
    (:`ForceSound`
      (`/Game/Insider/Blueprints/Core/BPM_CoreEngine.GE_3DSound` _handleopensound false _handleopensound (`self.HandlePivot`) (`self.Attenuation`)))))

(event `self.Open/On`
  (params (GameEvent :type Boolean))
  ;[1 1 1] Open / On
  (`/Game/Insider/Blueprints/Core/BPM_CoreEngine.GE_CheckInteraction`)
  (if (`self.Open`)
    (`self.ToggleDoor`)
    (elif (`self.Locked`)
      (`self.ForceDoor`)
      (else
        (`self.OpenHandle`)))))

(fn `UserConstructionScript`
  (`self.SetupSettings` (`self.CreateGameEvents`) (`self.Trigger Settings`) (`self.Mesh Settings`) (struct) (struct) (`self.Door Settings`) (`self.SoundAttenuation`)) ; Setup Parent Variables
  (`parent.UserConstructionScript`) ; Initialize Parent Configurations
  ;[1 1 1] Initialize that BP Configurations
  (`/Game/Insider/Blueprints/Core/BP_Functions.PlayRate` (`self.OpenCloseTimeline`) (`self.Door Open / Close Duration (Sec)`))
  (`/Game/Insider/Blueprints/Core/BP_Functions.PlayRate` (`self.HandleTimeline`) (`self.Handle Open / Release Duration (Sec)`))
  (`/Game/Insider/Blueprints/Core/BP_Functions.PlayRate` (`self.ForceTimeline`) (`self.ForceDuration (Sec)`))
  (`SceneComponent.K2_SetRelativeLocation` (`self.DoorPivot`) (select `bool` (`self.Open`) :`false` (`self.CloseLocation`) :`true` (`self.OpenLocation`)) false false)
  (`SceneComponent.K2_SetRelativeRotation` (`self.HandlePivot`) (select `bool` (`self.Open`) :`false` (`self.HandleReleaseRotation`) :`true` (`self.HandleOpenRotation`)) false false)
  (`TimelineComponent.SetNewTime` (`self.OpenCloseTimeline`) (select `bool` (`self.Open`) :`true` 1.0 :!type "Float (single-precision)"))
  (`SceneComponent.K2_AttachToComponent` (`self.LockPivot`) (`self.HandlePivot`) "None" "KeepWorld" "KeepWorld" "SnapToTarget" true))