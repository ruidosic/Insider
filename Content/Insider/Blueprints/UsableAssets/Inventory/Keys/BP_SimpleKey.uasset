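; BP_SimpleKey is a simple key usable asset for the inventory system, configured through exposed settings.
; Its construction script passes trigger, mesh, key, inspection, inventory and game event settings to SetupSettings, then runs the parent construction script.
; The event graph holds only disabled stub events, so this Blueprint adds no runtime logic of its own.
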(fn `UserConstructionScript`
  (`self.SetupSettings` (`self.Trigger Settings`) (`self.SimpleKeyMesh`) (`self.KeySettings`) (`self.Inspection Settings`) (`self.Inventory Settings`) (`self.CreateGameEvents`))
  (`parent.UserConstructionScript`))