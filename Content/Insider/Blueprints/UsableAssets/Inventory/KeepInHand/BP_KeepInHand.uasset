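; Base Blueprint for usable keep-in-hand equipment (flashlight, glowstick, torch, gun) that can be inspected and taken into main equipment.
; Use or inspection use takes it once if Takeable, otherwise Use falls back to alternative use, which begins inspection.
; CheckClass routes to the player's matching take function and GameEventCheck, then optionally shows an added-to-equipment notice.
; Only Flashlight resolves: the Glowstick check repeats BP_Flashlight, and Torch and Gun classes are unset.
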(event `self.AlternativeUse`
  (params (GameEvent :type Boolean))
  ;[1 1 1] Altrnative Use Events
  (if (not GameEvent)
    (`self.BeginInspection`)))

(event `self.InspectionAlternativeUse`
  ;[1 1 1] Altrnative Use Events
  (`self.EndInspection` false))

(event `self.Use`
  (params (GameEvent :type Boolean))
  ;[1 1 1] Use Events
  (if (`self.Takeable`)
    (`/Engine/EditorBlueprintResources/StandardMacros.DoOnce` false :!label _label
      (:`Completed`
        (`self.Take` true)
        (bind _as_core_engine (`/Game/Insider/Blueprints/Core/BP_Functions.GetPlayer`))
        (`self.CheckClass`
          (:`Flashlight`
            (`/Game/Insider/Blueprints/Core/BP_CoreEngine.TakeFlashlight` _as_core_engine)
            (`self.GameEventCheck` "NewEnumerator28"))
          (:`Glowstick`
            (`/Game/Insider/Blueprints/Core/BP_CoreEngine.TakeGlowstick` _as_core_engine)
            (`self.GameEventCheck` "NewEnumerator31"))
          (:`Torch`
            (`/Game/Insider/Blueprints/Core/BP_CoreEngine.TakeTorch` _as_core_engine)
            (`self.GameEventCheck` "NewEnumerator29"))
          (:`Gun`
            (`/Game/Insider/Blueprints/Core/BP_CoreEngine.TakeGun` _as_core_engine)
            (`self.GameEventCheck` "NewEnumerator30")))
        (if (`self.NoticedAboutAdd`)
          (`/Game/Insider/Blueprints/Core/BP_Functions.Notice` (`self.ItemName`) "" "added to equipment"))))
    (else
      (`self.AlternativeUse` GameEvent))))

(event `self.InspectionUse`
  ;[1 1 1] Use Events
  (if (`self.Takeable`)
    (goto _label)))

(fn `SetupSettings`
  (params (MeshSettings :type "/Game/Insider/Blueprints/UsableAssets/Structs/Struct_SetMesh Structure") (InspectionSettings :type "/Game/Insider/Blueprints/UsableAssets/Structs/Struct_InspectionSettings Structure") (GameEvent :type "Array of /Game/Insider/Blueprints/Events/Structs/Struct_GameEvents Structure") (NoticedAboutAdd :type Boolean))
  (set `self.MeshSettings` MeshSettings)
  (set `self.GameEvents` GameEvent)
  (set `self.NoticedAboutAdd` NoticedAboutAdd)
  (`self.SetInspection` InspectionSettings))

(fn `UserConstructionScript`
  (`parent.UserConstructionScript`))