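; BP_SimplePortal is a child portal Blueprint that exposes a basic configuration for a portal linked to a target portal.
; Its construction script copies its surface size, render, open-state and target variables into the portal through setters in SetupCoreVariables.
; It then runs the parent construction script, so these values are applied before the inherited setup executes.
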(fn `UserConstructionScript`
  (`self.SetMeshSurfaceSize` (`self.SurfaceMeshSize`))
  (`self.SetIsRenderEnable` (`self.RenderEnable`))
  (`self.SetIsOpen` (`self.Open`))
  (`self.SetTarget` (`self.Target Portal`))
  (`parent.UserConstructionScript`))