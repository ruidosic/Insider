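; Weight-sensitive trigger volume that fires game events based on the total mass of physics objects inside it.
; Overlaps with BP_PhysicsObject actors adjust a running weight by mesh mass, calling GameEventCheck with different values when MaxWeight is reached or lost.
; The exit that drops below the threshold fires its event without subtracting that object's mass.
; The construction script sizes the trigger box from TriggerSize.
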(event `self.OverlapTrigger.OnComponentBeginOverlap`
  (params (OverlappedComponent :type "PrimitiveComponent Object Reference") (OtherActor :type "Actor Object Reference") (OtherComp :type "PrimitiveComponent Object Reference") (OtherBodyIndex :type Integer) (bFromSweep :type Boolean) (SweepResult :type "HitResult Structure (by ref)"))
  ;[1 1 1] Begin Overlap
  (bind _asbp_physics_object (cast `/Game/Insider/Blueprints/UsableAssets/PhysicsObjects/BP_PhysicsObject` OtherActor))
  (if (< (`self.CurrentWeight`) (`self.MaxWeight`))
    (bind _returnvalue (+ (`self.CurrentWeight`) (`PrimitiveComponent.GetMass` (`/Game/Insider/Blueprints/UsableAssets/PhysicsObjects/BP_PhysicsObject.ObjectMesh` _asbp_physics_object))))
    (set `self.CurrentWeight` _returnvalue)
    (if (>= (`self.CurrentWeight`) (`self.MaxWeight`))
      (`self.GameEventCheck` "NewEnumerator26"))
    (else
      (set `self.CurrentWeight` _returnvalue))))

(event `self.OverlapTrigger.OnComponentEndOverlap`
  (params (OverlappedComponent :type "PrimitiveComponent Object Reference") (OtherActor :type "Actor Object Reference") (OtherComp :type "PrimitiveComponent Object Reference") (OtherBodyIndex :type Integer))
  ;[1 1 1] End Overlap
  (bind _asbp_physics_object (cast `/Game/Insider/Blueprints/UsableAssets/PhysicsObjects/BP_PhysicsObject` OtherActor))
  (bind _returnvalue (- (`self.CurrentWeight`) (`PrimitiveComponent.GetMass` (`/Game/Insider/Blueprints/UsableAssets/PhysicsObjects/BP_PhysicsObject.ObjectMesh` _asbp_physics_object))))
  (if (and (< _returnvalue (`self.MaxWeight`)) (>= (`self.CurrentWeight`) (`self.MaxWeight`)))
    (`self.GameEventCheck` "NewEnumerator27")
    (else
      (set `self.CurrentWeight` _returnvalue))))

(fn `UserConstructionScript`
  (`parent.UserConstructionScript`)
  (`BoxComponent.SetBoxExtent` (`self.OverlapTrigger`) (`self.TriggerSize`) true))