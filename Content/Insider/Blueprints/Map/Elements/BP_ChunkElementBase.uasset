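; Base Blueprint for map chunk elements, configured entirely in its construction script.
; It derives the element size from the static mesh bounds and fits the PlatformDetect box to the scaled X/Y footprint, with fixed height and a downward offset.
; An optional side shuffle randomizes axis order, rotating both meshes in quarter-turn multiples for visual variety.
; The jump trigger sizing step is an empty stub.
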(fn `GetStaticMeshHalfSize`
  (returns (Size :type "Vector Structure"))
  (return (`.BoxExtent` (`KismetMathLibrary.BreakBoxSphereBounds` (`StaticMesh.GetBounds` (`StaticMeshComponent.StaticMesh` (`self.ElementMesh`)))))))

(fn `ShuffleSide`
  (locals (Enum_RotationCoordinate :type "Array of /Game/Insider/Blueprints/Map/Enums/Enum_RotationCoordinate Enum"))
  (bind _elementskeletalmesh (`self.ElementSkeletalMesh`))
  (if (`self.ShuffleSide?`)
    (`KismetArrayLibrary.Array_Shuffle` (`local.Enum_RotationCoordinate`))
    (for (_array_element _array_index) (`local.Enum_RotationCoordinate`)
      (switch `/Game/Insider/Blueprints/Map/Enums/Enum_RotationCoordinate` _array_element
        (:`NewEnumerator0`
          (bind _returnvalue (* _array_index 90.0))
          (`SceneComponent.K2_AddRelativeRotation` _elementskeletalmesh (`KismetMathLibrary.MakeRotator` _returnvalue) false false)
          (`SceneComponent.K2_AddRelativeRotation` (`self.ElementMesh`) (`KismetMathLibrary.MakeRotator` _returnvalue) false false))
        (:`NewEnumerator1`
          (`SceneComponent.K2_AddRelativeRotation` _elementskeletalmesh (`KismetMathLibrary.MakeRotator` 0.0 _returnvalue) false false)
          (`SceneComponent.K2_AddRelativeRotation` (`self.ElementMesh`) (`KismetMathLibrary.MakeRotator` 0.0 _returnvalue) false false))
        (:`NewEnumerator2`
          (`SceneComponent.K2_AddRelativeRotation` _elementskeletalmesh (`KismetMathLibrary.MakeRotator` 0.0 0.0 _returnvalue) false false)
          (`SceneComponent.K2_AddRelativeRotation` (`self.ElementMesh`) (`KismetMathLibrary.MakeRotator` 0.0 0.0 _returnvalue) false false))))))

(fn `UserConstructionScript`
  (set `self.ElementSize` (* (`self.GetStaticMeshHalfSize`) 2)))