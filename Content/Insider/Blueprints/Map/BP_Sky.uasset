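; BP_Sky is a map sky actor with an optional, repeating lightning effect in its material.
; The construction script applies a dynamic instance of MISky to the mesh and, when Lightning is enabled, sets speed, intensity and timeline play rate from its variables.
; From BeginPlay, a self-calling event toggles the material's Multiply parameter, using LightningTimeline as the off interval and a Delay as the flash duration.
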(event `self.ReceiveBeginPlay`
  (`self.Lightning`))

(event `Lightning`
  (if (`self.Lightning?`)
    ;[1 1 1] Lightning Off
    (`MaterialInstanceDynamic.SetScalarParameterValue` (`self.DynMat_Sky`) "Multiply" 0.0)
    (`Timeline|LightningTimeline` :!via `PlayFromStart`
      (:`Finished`
        ;[1 1 1] Lightning On
        (`MaterialInstanceDynamic.SetScalarParameterValue` (`self.DynMat_Sky`) "Multiply" 1.0)
        (`KismetSystemLibrary.Delay` (`self.LightningDuration`))
        ;[1 1 1] Loop
        (`self.Lightning`)))))

(fn `UserConstructionScript`
  (bind _returnvalue (`KismetMaterialLibrary.CreateDynamicMaterialInstance` (`self.MI_Sky`)))
  (`PrimitiveComponent.SetMaterial` (`self.StaticMeshComponent`) 0 _returnvalue)
  (set `self.DynMat_Sky` _returnvalue)
  (if (`self.Lightning?`)
    (`MaterialInstanceDynamic.SetScalarParameterValue` (`self.DynMat_Sky`) "LightningSpeed" (`self.LightningSpeed`))
    (`/Game/Insider/Blueprints/Core/BP_Functions.PlayRate` (`self.LightningTimeline`) (`self.LightningDelay(Sec)`))
    (`MaterialInstanceDynamic.SetScalarParameterValue` (`self.DynMat_Sky`) "Lightning Intensity" (`self.LightningIntensity`))))