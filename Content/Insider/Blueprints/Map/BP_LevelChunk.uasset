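; BP_LevelChunk is a map piece built from a grid of mesh elements that can fall away.
; The construction script reads StructChunk, spawns mesh components with per-index overrides and optional shuffled 90-degree-step rotations, then fits a box collision around the grid.
; FallingDown walks the elements forward or reversed with a delay, either enabling physics directly or lowering each by timeline before optionally enabling physics.
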(event `/Game/Insider/Blueprints/Map/BPI_Chunk.FallingDown`
  (params (`Chunk Fall Seq` :type "/Game/Insider/Blueprints/Events/Structs/Struct_GE_ChunkFallSequence Structure"))
  (bind ((`Reverse_21_1F703C58461C5B8C3F69038A40E7A49F` _reverse) (`Smooth_19_B7E89DE643D81B33E6CE8890FEA3BCAE` _smooth) (`PhysicsSimulate_11_7E1AD90F481910C56727E08ECE0A4E86` _physicssimulate) (`SlowDown_10_F0B6586B46C7989478768CB565BF1A50` _slowdown) (`DownPointZ_22_85DA6CD1486D00D3C64BBBBFCDDAFF3A` _downpointz) (`DelayBetweenSeq_15_599C4B6A43C5086D5F177A9C5CCCF05F` _delaybetweenseq)) (break `/Game/Insider/Blueprints/Events/Structs/Struct_GE_ChunkFallSequence` `Chunk Fall Seq`))
  ;[1 1 1] FallingDown
  (if _slowdown
    (`self.FallMove` _reverse _smooth _delaybetweenseq _downpointz _physicssimulate)
    (else
      (`self.Simulate Physics` _reverse _delaybetweenseq))))

(event `FallMove`
  (params (Reverse :type Boolean) (Smooth :type Boolean) (Delay :type "Float (double-precision)") (`Down Point` :type "Float (double-precision)") (`Simulate Physics` :type Boolean))
  (bind _elementsref (`self.ElementsRef`))
  ;[1 1 1] Falling Move
  (if Reverse
    (bind (_array_index _array_element) (`/Game/Insider/Blueprints/Core/BPM_CoreEngine.ReverseForEachLoopWithDelay` _elementsref Delay)
      (:`Loop Body`
        (`/Engine/EditorBlueprintResources/StandardMacros.IsValid` _array_element
          (:`Is Valid`
            (set `self.CurrentMeshLocation` (`SceneComponent.K2_GetComponentLocation` _array_element))))))
    (else
      (bind _arrayelement (`/Game/Insider/Blueprints/Core/BPM_CoreEngine.ForEachLoopWithDelay` _elementsref Delay)
        (:`Loop Body`
          (`/Engine/EditorBlueprintResources/StandardMacros.IsValid` _arrayelement
            (:`Is Valid`
              (set `self.CurrentMeshLocation` (`SceneComponent.K2_GetComponentLocation` _arrayelement))))))))
  (`TimelineComponent.SetPlayRate` (`self.FallTimeline`) (- Delay 0.1))
  (bind (_direction _linear _smooth) (`Timeline|FallTimeline` :!via `PlayFromStart`)
    (:`Update`
      (`SceneComponent.K2_SetWorldLocation` (select `bool` Reverse :`false` _arrayelement :`true` _array_element) (`KismetMathLibrary.MakeVector` (.x (`self.CurrentMeshLocation`)) (.y (`self.CurrentMeshLocation`)) (`KismetMathLibrary.Lerp` (.z (`self.CurrentMeshLocation`)) (- 0.0 `Down Point`) (select `bool` Smooth :`false` _linear :`true` _smooth))) false false))
    (:`Finished`
      (`PrimitiveComponent.SetSimulatePhysics` (select `bool` Reverse :`false` _arrayelement :`true` _array_element :!type "PrimitiveComponent Object Reference") `Simulate Physics`))))

(event `Simulate Physics`
  (params (Reverse :type Boolean) (Delay :type "Float (double-precision)"))
  (bind _elementsref (`self.ElementsRef`))
  ;[1 1 1] Simulate Physics
  (if Reverse
    (bind (_array_index _array_element) (`/Game/Insider/Blueprints/Core/BPM_CoreEngine.ReverseForEachLoopWithDelay` _elementsref Delay)
      (:`Loop Body`
        (`/Engine/EditorBlueprintResources/StandardMacros.IsValid` _array_element
          (:`Is Valid`
            (`PrimitiveComponent.SetSimulatePhysics` _array_element true)))))
    (else
      (bind _arrayelement (`/Game/Insider/Blueprints/Core/BPM_CoreEngine.ForEachLoopWithDelay` _elementsref Delay)
        (:`Loop Body`
          (`/Engine/EditorBlueprintResources/StandardMacros.IsValid` _arrayelement
            (:`Is Valid`
              (`PrimitiveComponent.SetSimulatePhysics` _arrayelement true))))))))

(fn `CalculateChunkLength`
  (returns (ReturnValue :type "Float (double-precision)"))
  (bind _output (`|GetArrayItem` (`self.ElementsRef`)))
  (return (+ (* (`self.Length`) (.x (select `bool` (`KismetSystemLibrary.IsValid` _output) :`true` (* (`self.GetExtendHalfSize` _output) 2)))) (* (- (`self.Length`) 1) (`self.DistanceBetween`)))))

(fn `CalculateChunkWidth`
  (returns (ReturnValue :type "Float (double-precision)"))
  (bind _output (`|GetArrayItem` (`self.ElementsRef`)))
  (return (+ (* (`self.Width`) (.y (select `bool` (`KismetSystemLibrary.IsValid` _output) :`true` (* (`self.GetExtendHalfSize` _output) 2)))) (* (- (`self.Width`) 1) (`self.DistanceBetween`)))))

(fn `GetExtendHalfSize`
  (params (StaticMeshComponent :type "StaticMeshComponent Object Reference"))
  (returns (`Box Extent` :type "Vector Structure"))
  (return (`.BoxExtent` (`KismetMathLibrary.BreakBoxSphereBounds` (`StaticMesh.GetBounds` (`StaticMeshComponent.StaticMesh` StaticMeshComponent))))))

(fn `ShuffleSides`
  (params (`Shuffle?` :type Boolean) (StaticMesh :type "StaticMeshComponent Object Reference"))
  (locals (Enum_RotationCoordinate :type "Array of /Game/Insider/Blueprints/Map/Enums/Enum_RotationCoordinate Enum"))
  (if `Shuffle?`
    (`/Engine/EditorBlueprintResources/StandardMacros.IsValid` StaticMesh
      (:`Is Valid`
        (`KismetArrayLibrary.Array_Shuffle` (`local.Enum_RotationCoordinate`))
        (for (_array_element _array_index) (`local.Enum_RotationCoordinate`)
          (switch `/Game/Insider/Blueprints/Map/Enums/Enum_RotationCoordinate` _array_element
            (:`NewEnumerator0`
              (bind _returnvalue (* _array_index 90.0))
              (`SceneComponent.K2_AddRelativeRotation` StaticMesh (`KismetMathLibrary.MakeRotator` _returnvalue) false false))
            (:`NewEnumerator1`
              (`SceneComponent.K2_AddRelativeRotation` StaticMesh (`KismetMathLibrary.MakeRotator` 0.0 _returnvalue) false false))
            (:`NewEnumerator2`
              (`SceneComponent.K2_AddRelativeRotation` StaticMesh (`KismetMathLibrary.MakeRotator` 0.0 0.0 _returnvalue) false false))))))))

(fn `UserConstructionScript`
  (bind (_dimension _collision _totalelements _specialelementmesh) (break `/Game/Insider/Blueprints/Map/Structs/Struct_Chunk` (`self.Struct_Chunk`)))
  (bind (_elementmesh _elementmaterial) (break `/Game/Insider/Blueprints/Map/Structs/Struct_C_Element` (`self.TotalElement`)))
  (bind (_length _width _distancebetween) (break `/Game/Insider/Blueprints/Map/Structs/Struct_C_Dimension` _dimension))
  (bind (_chunkcollisionmultiplier _chunkcollisionheight) (break `/Game/Insider/Blueprints/Map/Structs/Struct_C_Collision` _collision))
  (set `self.Length` _length)
  (set `self.Width` _width)
  (set `self.DistanceBetween` _distancebetween)
  (set `self.ChunkCollisionMultiplier` _chunkcollisionmultiplier)
  (set `self.ChunkCollisionHeight` _chunkcollisionheight)
  (set `self.TotalElement` _totalelements)
  (set `self.SpecialElement` _specialelementmesh)
  (`KismetArrayLibrary.Array_Clear` (`self.SpawnStartPoints`))
  (`KismetArrayLibrary.Array_Clear` (`self.ElementsRef`))
  (for _index (range (`self.Length`))
    (for _index_2 (range (`self.Width`))
      (bind _returnvalue (`AddComponent|NODE_AddStaticMeshComponent-1`))
      (bind _returnvalue_2 (+ (* _index (`self.Width`)) _index_2))
      (bind (_value _returnvalue_3) (`BlueprintMapLibrary.Map_Find` (`self.SpecialElement`) _returnvalue_2))
      (bind _returnvalue_4 (select `bool` _returnvalue_3 :`false` _elementmesh :`true` (break `/Game/Insider/Blueprints/Map/Structs/Struct_C_Element` _value)))
      (`/Engine/EditorBlueprintResources/StandardMacros.IsValid` _returnvalue_4
        (:`Is Valid`
          (`PrimitiveComponent.SetMaterial` _returnvalue 0 (select `bool` _returnvalue_3 :`false` _elementmaterial :`true` (`.ElementMaterial_14_0C836A314DED90D2B81E70BD3A9176D6` (break `/Game/Insider/Blueprints/Map/Structs/Struct_C_Element` _value))))
          (`StaticMeshComponent.SetStaticMesh` _returnvalue _returnvalue_4)
          (bind (_value_2 _returnvalue_5) (`BlueprintMapLibrary.Map_Find` (`self.SpecialElement`) _returnvalue_2))
          (`self.ShuffleSides` (select `bool` _returnvalue_5 :`false` (`.ShuffleSides?_12_203836664773C4C80FD60C8CC081B16C` (break `/Game/Insider/Blueprints/Map/Structs/Struct_C_Element` (`self.TotalElement`))) :`true` (`.ShuffleSides?_12_203836664773C4C80FD60C8CC081B16C` (break `/Game/Insider/Blueprints/Map/Structs/Struct_C_Element` _value_2))) _returnvalue)
          (`KismetArrayLibrary.Array_Add` (`self.ElementsRef`) _returnvalue)
          (bind _result (`self.CalculateStartLocation` _index_2 _index (`self.GetExtendHalfSize` _returnvalue)))
          (`KismetArrayLibrary.Array_Add` (`self.SpawnStartPoints`) _result)
          (`SceneComponent.K2_SetWorldLocation` _returnvalue _result false false)
          (`SceneComponent.K2_SetWorldLocation` (`self.ChunkCollision`) (- (+ (`SceneComponent.K2_GetComponentLocation` (`self.DefaultSceneRoot`)) (`KismetMathLibrary.MakeVector` (/ (`self.CalculateChunkLength`) 2.0) (/ (`self.CalculateChunkWidth`) 2.0))) (`self.GetExtendHalfSize` (`|GetArrayItem` (`self.ElementsRef`)))) false false)
          (`BoxComponent.SetBoxExtent` (`self.ChunkCollision`) (* (`KismetMathLibrary.MakeVector` (/ (`self.CalculateChunkLength`) 2.0) (/ (`self.CalculateChunkWidth`) 2.0) (`self.ChunkCollisionHeight`)) (`self.ChunkCollisionMultiplier`)) true))
        (:`Is Not Valid`
          (`ActorComponent.K2_DestroyComponent` _returnvalue))))))